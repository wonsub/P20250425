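; BP_PlayerState tracks the player's health in the HackAndSlash game, using CurHP and MaxHP.
; AddDamage subtracts damage from CurHP and broadcasts UpdatePlayerHP with the current and maximum values.
; IsDeath is checked before subtracting, so PlayerDeath fires only on a damage call made when HP is already at or below zero, not on the killing blow.
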(fn `AddDamage`
  (params (Damage :type "Float (double-precision)"))
  (if (`self.IsDeath`)
    (`self.EventDispatcher_PlayerDeath`)
    (else
      (bind _output_get (set `self.CurHP` (- (`self.CurHP`) Damage)))
      (`self.EventDispatcher_UpdatePlayerHP` _output_get (`self.MaxHP`)))))

(fn `IsDeath`
  (returns (IsDeath :type Boolean))
  (return (<= (`self.CurHP`) 0.0)))

(fn `UserConstructionScript`)