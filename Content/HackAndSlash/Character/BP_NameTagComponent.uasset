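; BP_NameTagComponent is an actor component that gives its owner an on-screen name tag showing a name and health.
; On BeginPlay it creates a name tag widget, passes itself as a reference, and adds it to the viewport.
; SetName and SetHP forward values to that widget, and EndPlay removes it from its parent.
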(event `self.ReceiveBeginPlay`
  (bind _returnvalue (`|CreateWidget` "/Game/HackAndSlash/Character/NameTagWidget.NameTagWidget_C" null self))
  (bind _output_get (set `self.NameTag` _returnvalue))
  (`UserWidget.AddToViewport` _output_get 0))

(event `self.ReceiveEndPlay`
  (params (EndPlayReason :type "EEndPlayReason Enum" :default "Destroyed"))
  (`Widget.RemoveFromParent` (`self.NameTag`)))

(fn `SetHP`
  (params (CurHP :type "Float (single-precision)") (MaxHP :type "Float (double-precision)"))
  (`/Game/HackAndSlash/Character/NameTagWidget.SetHP` (`self.NameTag`) CurHP MaxHP))

(fn `SetName`
  (params (Name :type String))
  (`/Game/HackAndSlash/Character/NameTagWidget.SetName` (`self.NameTag`) Name))