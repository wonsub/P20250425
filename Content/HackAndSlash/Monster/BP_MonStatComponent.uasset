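; BP_MonStatComponent is an actor component that holds a monster's stats and current HP.
; SetMonStat loads a row from DT_Monster by name, starts current HP at MaxHP and broadcasts the MonStat dispatcher.
; AddDamage subtracts HP while the monster is alive, fires UpdateHP, and fires Death when HP drops to zero or below, with IsDeath exposing that check.
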(fn `AddDamage`
  (params (Damage :type "Float (double-precision)"))
  (bind (_curmonstate_monstate _curmonstate_curhp) (break `/Game/HackAndSlash/Monster/ST_CurMonState` (`self.CurMonState`)))
  (bind _curmonstate (`self.CurMonState`))
  (if (not (`self.IsDeath`))
    (bind _structout (setmembers `/Game/HackAndSlash/Monster/ST_CurMonState` :`StructRef` (`self.CurMonState`) :`CurHP` (- _curmonstate_curhp Damage)))
    (`self.EventDispatcher_UpdateHP` (`.CurHP_5_C14F97544B1E24B5A3BE808122A11223` (break `/Game/HackAndSlash/Monster/ST_CurMonState` _curmonstate)) (`.MaxHP_8_92FB746349D1CDF5305F7CA3B6A86A65` (break `/Game/HackAndSlash/Monster/ST_MonState` (break `/Game/HackAndSlash/Monster/ST_CurMonState` _curmonstate))))
    (if (<= (`.CurHP_5_C14F97544B1E24B5A3BE808122A11223` (break `/Game/HackAndSlash/Monster/ST_CurMonState` _structout)) 0.0)
      (`self.EventDispatcher_Death` (`self.CurMonState`)))))

(fn `IsDeath`
  (returns (IsDead :type Boolean))
  (bind (_curmonstate_monstate _curmonstate_curhp) (break `/Game/HackAndSlash/Monster/ST_CurMonState` (`self.CurMonState`)))
  (return (<= _curmonstate_curhp 0.0)))

(fn `SetMonStat`
  (params (RowName :type Name))
  (bind _returnvalue (`|GetDataTableRow` "/Game/HackAndSlash/Monster/DT_Monster.DT_Monster" RowName)
    (:`then`
      (bind _output_get (set `self.CurMonState` (make `/Game/HackAndSlash/Monster/ST_CurMonState` _returnvalue (`.MaxHP_8_92FB746349D1CDF5305F7CA3B6A86A65` (break `/Game/HackAndSlash/Monster/ST_MonState` _returnvalue)))))
      (`self.EventDispatcher_MonStat` _output_get))))