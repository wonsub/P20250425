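; Actor component that periodically spawns random monsters around its owner in the hack-and-slash game.
; A looping one-second timer picks a random offset from the owner, scaled by Radius times pi with independent X and Y angles.
; If an object trace from that point hits world geometry, it spawns a random DT_Monster class with BT_AIMon and applies that row's stats.
; The trace end subtracts a second random world location from the start.
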(event `self.ReceiveBeginPlay`
  (`KismetSystemLibrary.K2_SetTimer` null "DoSpawn" 1.0 true))

(fn `DoSpawn`
  (locals (RandLocation :type "Vector Structure" :default (0.0 0.0 0.0)) (RandName :type Name))
  (bind _output_get (set `local.RandLocation` (`self.GetRandomCircleLocation`)))
  (if (`self.IsCanSpawn` _output_get)
    (bind _outrownames (`DataTableFunctionLibrary.GetDataTableRowNames` "/Game/HackAndSlash/Monster/DT_Monster.DT_Monster"))
    (bind _output_get_2 (set `local.RandName` (`KismetArrayLibrary.Array_Random` _outrownames)))
    (bind _returnvalue (`|GetDataTableRow` "/Game/HackAndSlash/Monster/DT_Monster.DT_Monster" _output_get_2)
      (:`then`
        (bind _returnvalue_2 (`AIBlueprintHelperLibrary.SpawnAIFromClass` (`.MonsterClass_12_4DC0F19648B9EA149F8014A6EA8A0AA6` (break `/Game/HackAndSlash/Monster/ST_MonState` _returnvalue)) "/Game/HackAndSlash/AI/BT_AIMon.BT_AIMon" (`local.RandLocation`) (struct) false null))
        (bind _asbp_monster_base (cast `/Game/HackAndSlash/Monster/BP_MonsterBase` _returnvalue_2))
        (`/Game/HackAndSlash/Monster/BP_MonsterBase.SetMonStat` _asbp_monster_base (`local.RandName`))))))

(fn `GetRandomCircleLocation`
  (returns (RandLocation :type "Vector Structure"))
  (locals (Radius :type "Float (double-precision)" :default 250.0))
  (bind _returnvalue (`KismetMathLibrary.RandomFloatInRange` 0.0 360.0))
  (bind _returnvalue_2 (* (`local.Radius`) 3.141592))
  (set `self.Rand` _returnvalue)
  (return (+ (`Actor.K2_GetActorLocation` (`self.GetOwner`)) (`KismetMathLibrary.MakeVector` (* (`KismetMathLibrary.Cos` _returnvalue) _returnvalue_2) (* (`KismetMathLibrary.Sin` _returnvalue) _returnvalue_2)))))

(fn `IsCanSpawn`
  (params (WorldLocation :type "Vector Structure"))
  (returns (ReturnValue :type Boolean))
  (bind (_outhits _returnvalue) (`KismetSystemLibrary.LineTraceMultiForObjects` WorldLocation (- WorldLocation (`self.GetRandomCircleLocation`)) (`|MakeArray` "ObjectTypeQuery1" "ObjectTypeQuery2" :!type "EObjectTypeQuery Enum")))
  (return _returnvalue))